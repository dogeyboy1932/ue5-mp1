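; BP_Tunnel is an endless-runner tunnel segment with a rotating holed wall, a health pack and an enemy.
; Wall and enemy damage non-phasing players; projectiles hitting enemies award score and collection, and ten collections unlock phasing, as do health pickups.
; Crossing the trigger adds score, has TunnelSpawner spawn another segment and destroys this one.
; Randomize functions vary wall shape, roll and item offsets, but nothing here calls them.
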(event `self.ReceiveTick`
  (params (DeltaSeconds :type "Float (single-precision)"))
  (`SceneComponent.K2_AddLocalRotation` (`self.WallMesh`) (`KismetMathLibrary.MakeRotator` (* DeltaSeconds (`self.RotateSpeed`))) false false))

(event `self.WallMesh.OnComponentBeginOverlap`
  (params (OverlappedComponent :type "PrimitiveComponent Object Reference") (OtherActor :type "Actor Object Reference") (OtherComp :type "PrimitiveComponent Object Reference") (OtherBodyIndex :type Integer) (bFromSweep :type Boolean) (SweepResult :type "HitResult Structure (by ref)"))
  (bind _asbp_player (cast `/Game/InfiniteMatrix/Blueprints/BP_Player` OtherActor)
    (:`then`
      (if (not (`/Game/InfiniteMatrix/Blueprints/BP_Player.isPhasing` _asbp_player))
        (`|ExecutionSequence`
          (:`then_0`
            (bind _output_get (set `/Game/InfiniteMatrix/Blueprints/BP_Player.Health` (- (`/Game/InfiniteMatrix/Blueprints/BP_Player.Health` _asbp_player) 20.0) _asbp_player))
            (`|ExecutionSequence`
              (:`then_1`
                (if (<= _output_get 0.0)
                  (set `/Game/InfiniteMatrix/Blueprints/BP_Player.IsDead` true _asbp_player)
                  (`/Game/InfiniteMatrix/Blueprints/BP_Player.DisplayRestart` _asbp_player)))))
          (:`then_1`
            (set `/Game/InfiniteMatrix/Blueprints/BP_Player.Score` (- (`/Game/InfiniteMatrix/Blueprints/BP_Player.Score` _asbp_player) 1.0) _asbp_player)))))
    (:`CastFailed`
      (bind _asbp_projectile (cast `/Game/InfiniteMatrix/Blueprints/BP_Projectile` OtherActor))
      (`self.K2_DestroyActor` _asbp_projectile))))

(event `self.TriggerZone.OnComponentBeginOverlap`
  (params (OverlappedComponent :type "PrimitiveComponent Object Reference") (OtherActor :type "Actor Object Reference") (OtherComp :type "PrimitiveComponent Object Reference") (OtherBodyIndex :type Integer) (bFromSweep :type Boolean) (SweepResult :type "HitResult Structure (by ref)"))
  (bind _asbp_player (cast `/Game/InfiniteMatrix/Blueprints/BP_Player` OtherActor))
  (`|ExecutionSequence`
    (:`then_0`
      (`/Game/InfiniteMatrix/Blueprints/BP_TunnelSpawner.SpawnTunnelAtSpawnPoint` (`self.TunnelSpawner`))
      (`self.K2_DestroyActor`))
    (:`then_1`
      (set `/Game/InfiniteMatrix/Blueprints/BP_Player.Score` (+ (`/Game/InfiniteMatrix/Blueprints/BP_Player.Score` _asbp_player) 1.0) _asbp_player))))

(event `self.HealthPack.OnComponentBeginOverlap`
  (params (OverlappedComponent :type "PrimitiveComponent Object Reference") (OtherActor :type "Actor Object Reference") (OtherComp :type "PrimitiveComponent Object Reference") (OtherBodyIndex :type Integer) (bFromSweep :type Boolean) (SweepResult :type "HitResult Structure (by ref)"))
  (bind _asbp_player (cast `/Game/InfiniteMatrix/Blueprints/BP_Player` OtherActor))
  (`|ExecutionSequence`
    (:`then_0`
      (set `/Game/InfiniteMatrix/Blueprints/BP_Player.Health` (`KismetMathLibrary.Conv_IntToDouble` (`KismetMathLibrary.Min` (+ (`/Game/InfiniteMatrix/Blueprints/BP_Player.Health` _asbp_player) 10) (`KismetMathLibrary.FTrunc` (`/Game/InfiniteMatrix/Blueprints/BP_Player.Max Health` _asbp_player)))) _asbp_player))
    (:`then_1`
      (set `/Game/InfiniteMatrix/Blueprints/BP_Player.Collection` (+ (`/Game/InfiniteMatrix/Blueprints/BP_Player.Collection` _asbp_player) 1) _asbp_player))
    (:`then_2`
      (bind _collection (`/Game/InfiniteMatrix/Blueprints/BP_Player.Collection` _asbp_player))
      (if (>= _collection 10)
        (set `/Game/InfiniteMatrix/Blueprints/BP_Player.isPhasable` true _asbp_player)
        (`ActorComponent.K2_DestroyComponent` OverlappedComponent)
        (else
          (`KismetSystemLibrary.PrintString` (`KismetStringLibrary.Conv_IntToString` _collection)))))))

(event `self.EnemyMesh.OnComponentBeginOverlap`
  (params (OverlappedComponent :type "PrimitiveComponent Object Reference") (OtherActor :type "Actor Object Reference") (OtherComp :type "PrimitiveComponent Object Reference") (OtherBodyIndex :type Integer) (bFromSweep :type Boolean) (SweepResult :type "HitResult Structure (by ref)"))
  (bind _asbp_player (cast `/Game/InfiniteMatrix/Blueprints/BP_Player` OtherActor)
    (:`then`
      (if (`/Game/InfiniteMatrix/Blueprints/BP_Player.isPhasing` _asbp_player)
        (`KismetSystemLibrary.PrintString` "GHOSTED")
        (else
          (`|ExecutionSequence`
            (:`then_0`
              (bind _output_get (set `/Game/InfiniteMatrix/Blueprints/BP_Player.Health` (- (`/Game/InfiniteMatrix/Blueprints/BP_Player.Health` _asbp_player) 30.0) _asbp_player))
              (if (<= _output_get 0.0)
                (set `/Game/InfiniteMatrix/Blueprints/BP_Player.IsDead` true _asbp_player)
                (`/Game/InfiniteMatrix/Blueprints/BP_Player.DisplayRestart` _asbp_player))
              (`ActorComponent.K2_DestroyComponent` OverlappedComponent :!label _label))))))
    (:`CastFailed`
      (bind _asbp_projectile (cast `/Game/InfiniteMatrix/Blueprints/BP_Projectile` OtherActor))
      (bind _spawningplayer (`/Game/InfiniteMatrix/Blueprints/BP_Projectile.SpawningPlayer` _asbp_projectile))
      (set `/Game/InfiniteMatrix/Blueprints/BP_Player.Collection` (+ (`/Game/InfiniteMatrix/Blueprints/BP_Player.Collection` _spawningplayer) 1) _spawningplayer)
      (set `/Game/InfiniteMatrix/Blueprints/BP_Player.Score` (+ (`/Game/InfiniteMatrix/Blueprints/BP_Player.Score` _spawningplayer) 1.0) _spawningplayer)
      (if (>= (`/Game/InfiniteMatrix/Blueprints/BP_Player.Collection` _spawningplayer) 10)
        (set `/Game/InfiniteMatrix/Blueprints/BP_Player.isPhasable` true _spawningplayer))
      (`self.K2_DestroyActor` _asbp_projectile)
      (goto _label))))

(fn `RandomizeEnemy `
  (if (`KismetMathLibrary.RandomBoolWithWeight` 0.3)
    (`SceneComponent.K2_AddLocalOffset` (`self.EnemyMesh`) (`KismetMathLibrary.MakeVector` 0.0 (`KismetMathLibrary.RandomFloatInRange` -250.0 250.0) (`KismetMathLibrary.RandomFloatInRange` -250.0 250.0)) false true)))

(fn `RandomizeHealthpack`
  (`SceneComponent.K2_AddLocalOffset` (`self.HealthPack`) (`KismetMathLibrary.MakeVector` 0.0 (`KismetMathLibrary.RandomFloatInRange` -200.0 200.0) (`KismetMathLibrary.RandomFloatInRange` -200.0 200.0)) false true))

(fn `RandomizeWall`
  (`StaticMeshComponent.SetStaticMesh` (`self.WallMesh`) (select `int` (`KismetMathLibrary.RandomIntegerInRange` 0 3) :`0` "/Game/InfiniteMatrix/Meshes/SM_Hole_01.SM_Hole_01" :`1` "/Game/InfiniteMatrix/Meshes/SM_Hole_02.SM_Hole_02" :`2` "/Game/InfiniteMatrix/Meshes/SM_Hole_03.SM_Hole_03" :`3` "/Game/InfiniteMatrix/Meshes/SM_Hole_04.SM_Hole_04" :!type "StaticMesh Object Reference"))
  (`SceneComponent.K2_AddLocalRotation` (`self.WallMesh`) (`KismetMathLibrary.MakeRotator` (`KismetMathLibrary.RandomFloatInRange` 0.0 360.0)) false false))

(fn `UserConstructionScript`)